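; BP_Laser is an actor that displays a laser beam through a Niagara component.
; Each tick it writes its StartLocation and EndLocation variables to the effect's BeamStart and BeamEnd parameters, so the beam follows changes to those points.
; Its End event plays the Scale timeline, which drives the effect's Scale parameter and destroys the actor when finished.
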(event Custom|End
  (bind _newtrack_0 (Timeline|Scale Play)
    (:Update
      (Niagara|SetNiagaraVariable(Float) (Variables|Default|GetNiagara) "Scale" _newtrack_0))
    (:Finished
      (Actor|DestroyActor))))

(event EventBeginPlay)

(event Collision|EventActorBeginOverlap
  (params (OtherActor :type Actor%20Object%20Reference)))

(event EventTick
  (params (DeltaSeconds :type Float%20%28single-precision%29))
  (Niagara|SetNiagaraVariable(Vector3) (Variables|Default|GetNiagara) "BeamStart" (Variables|Default|GetStartLocation))
  (Niagara|SetNiagaraVariable(Vector3) (Variables|Default|GetNiagara) "BeamEnd" (Variables|Default|GetEndLocation)))

(fn ConstructionScript)