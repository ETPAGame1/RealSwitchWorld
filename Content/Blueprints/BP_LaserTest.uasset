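; BP_LaserTest is a test Blueprint that drives a laser beam effect from the first-person character's weapon socket.
; Each tick it sets the beam start to the EndLaser socket on SpawnProjectile and line-traces on Visibility toward a point DistanceInt along the camera's forward vector.
; The beam end snaps to the impact point on a hit, otherwise to the trace end, with the trace debug-drawn each frame.
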(event EventTick
  (params (DeltaSeconds :type Float%20%28single-precision%29))
  (bind _firstpersoncharacter (Variables|Default|GetFIrstPersonCharacter))
  (bind _spawn_projectile (Variables|/Game/Blueprints/BP_FirstPersonCharacter.BP_FirstPersonCharacter_C|GetSpawn_projectile _firstpersoncharacter))
  (bind _firstpersoncamera (Variables|/Game/Blueprints/BP_FirstPersonCharacter.BP_FirstPersonCharacter_C|GetFirstPersonCamera _firstpersoncharacter))
  (bind _returnvalue (Transformation|GetSocketLocation _spawn_projectile "EndLaser"))
  (Effects|Components|ParticleSystem|SetVectorParameter (Variables|Default|GetLaser) "USER.BeamStart" _returnvalue)
  (bind _outhit (Collision|LineTraceByChannel _returnvalue (+ (* (Math|Vector|GetForwardVector _firstpersoncamera) (Variables|Default|GetDistance%20Int)) (Transformation|GetWorldLocation _firstpersoncamera)) "TraceTypeQuery1" false 0 "ForOneFrame"))
  (Effects|Components|ParticleSystem|SetVectorParameter (Variables|Default|GetLaser) "USER.BeamEnd" (Math|Vector|SelectVector (.impactpoint _outhit) (.traceend _outhit) (Utilities|IsValid (.hitcomponent _outhit)))))

(fn ConstructionScript)