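; Laser-activated button that forwards an interact message to its linked objects, swaps its light material and plays a switch effect.
; CanStay checks the state flags of linked doors, turrets and traps; when it passes, the button sets Stayed and keeps its lit material.
; When the turret laser ends, it switches off linked cables and reruns the unlit-material path for each linked object.
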(event Custom|EndLaserTurret
  (for _array_element (Variables|Default|GetRefInteracted)
    (bind _asbp_cable (Utilities|Casting|CastToBP_Cable _array_element)
      (:then
        (Default|ButtonOff _asbp_cable))
      (:CastFailed
        (bind _asbp_cable_corner (Utilities|Casting|CastToBP_CableCorner _array_element)
          (:then
            (Default|ButtonOff _asbp_cable_corner))
          (:CastFailed
            _))))
    (Rendering|Material|SetMaterial (Variables|Default|GetStaticMesh) 0 "/Game/Materials/M_LumièrePorte.M_LumièrePorte")
    (Audio|Components|Audio|Play (Variables|Default|Getinterrupteur-actriver) 0.0)
    (bind _canstay_ (CallFunction|CanStay?))
    (if _canstay_
      (Variables|Default|SetStayed true)
      (Rendering|Material|SetMaterial (Variables|Default|GetStaticMesh) 0 "/Game/Materials/M_LumièrePorte_Inst.M_LumièrePorte_Inst"))))

(event EventLaserInteract
  (params (Active :type Boolean))
  (bind _staticmesh (Variables|Default|GetStaticMesh))
  (Variables|Default|SetActivated Active)
  (Class|BPIInteract|ButtonInteract(Message) (Variables|Default|GetRefInteracted))
  (if Active
    (Rendering|Material|SetMaterial _staticmesh 0 "/Game/Materials/M_LumièrePorte_Inst.M_LumièrePorte_Inst")
    (else
      (Rendering|Material|SetMaterial _staticmesh 0 "/Game/Materials/M_LumièrePorte.M_LumièrePorte")))
  (Audio|Components|Audio|Play (Variables|Default|Getinterrupteur-actriver) 0.0)
  (bind _canstay_ (CallFunction|CanStay?))
  (if _canstay_
    (Variables|Default|SetStayed true)
    (Rendering|Material|SetMaterial (Variables|Default|GetStaticMesh) 0 "/Game/Materials/M_LumièrePorte_Inst.M_LumièrePorte_Inst")))

(fn ConstructionScript)

(fn CanStay?
  (for _array_element (Variables|Default|GetRefInteracted)
    (bind _asbp_door_cool (Utilities|Casting|CastToBP_DoorCool _array_element)
      (:then
        (if (not (Variables|/Game/Blueprints/Objet_Interactable/BP_DoorCool.BP_DoorCool_C|GetRasLeCulDesBoolean _asbp_door_cool))
          (return false)))
      (:CastFailed
        (bind _asfbx_scene_turret_bottom_obj (Utilities|Casting|CastToFbxScene_Turret_Bottom_OBJ _array_element)
          (:then
            (if (not (Variables|/Game/Blueprints/Objet_Interactable/FbxScene_Turret_Bottom_OBJ.FbxScene_Turret_Bottom_OBJ_C|GetIsFiring? _asfbx_scene_turret_bottom_obj))
              (return false)))
          (:CastFailed
            (bind _asbp_trap (Utilities|Casting|CastToBP_Trap _array_element))
            (if (not (Variables|/Game/Blueprints/Objet_Interactable/BP_Trap.BP_Trap_C|GetOuais _asbp_trap))
              (return false)))))))
  (return true))

(fn ButtonInteract
  (return))