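; BP_Cable is an interactable-object cable whose light strip shows the state of its linked buttons.
; ButtonInteract applies the lit material instance when every entry in the Button array is Activated or, failing that, when every one is a BP_Button with Stayed set.
; Otherwise it applies the base material, which ButtonOff also restores unconditionally.
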(event Custom|ButtonOff
  (Rendering|Material|SetMaterial (Variables|Default|GetBandeLumineuse) 0 "/Game/Materials/M_LumièrePorte.M_LumièrePorte"))

(event EventButtonInteract
  (bind _m_enbatslescouilles (CallFunction|CanOpen?))
  (if _m_enbatslescouilles
    (Rendering|Material|SetMaterial (Variables|Default|GetBandeLumineuse) 0 "/Game/Materials/M_LumièrePorte_Inst.M_LumièrePorte_Inst")
    (else
      (Rendering|Material|SetMaterial (Variables|Default|GetBandeLumineuse) 0 "/Game/Materials/M_LumièrePorte.M_LumièrePorte")
      (bind _canstay_ (CallFunction|CanStay?))
      (if _canstay_
        (Rendering|Material|SetMaterial (Variables|Default|GetBandeLumineuse) 0 "/Game/Materials/M_LumièrePorte_Inst.M_LumièrePorte_Inst")
        (else
          (Rendering|Material|SetMaterial (Variables|Default|GetBandeLumineuse) 0 "/Game/Materials/M_LumièrePorte.M_LumièrePorte"))))))

(fn ConstructionScript)

(fn CanOpen?
  (for _array_element (Variables|Default|GetButton)
    (if (not (Variables|/Game/Blueprints/Objet_Interactable/BP_Button.BP_Button_C|GetActivated _array_element))
      (return false)))
  (return true))

(fn CanStay?
  (for _array_element (Variables|Default|GetButton)
    (bind _asbp_button (Utilities|Casting|CastToBP_Button _array_element))
    (if (not (Variables|/Game/Blueprints/Objet_Interactable/BP_Button.BP_Button_C|GetStayed _asbp_button))
      (return false)))
  (return true))