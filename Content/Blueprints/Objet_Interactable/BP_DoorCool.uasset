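; A door that slides up once every button linked to it is activated.
; The ButtonInteract event runs CanOpen, which checks the Activated state of each entry in the Button array.
; On success it plays an opening sound, sets a flag, switches the sphere to a door-light material and runs the half-speed Open timeline to raise the door mesh along Z.
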(event EventButtonInteract
  (bind _sm_door_l_staticmeshcomponent0 (Variables|Default|GetSM_Door_L_StaticMeshComponent0))
  (bind _relativelocation (Variables|/Script/Engine.SceneComponent|GetRelativeLocation _sm_door_l_staticmeshcomponent0))
  (bind _m_enbatslescouilles (CallFunction|CanOpen?))
  (if _m_enbatslescouilles
    (Audio|Components|Audio|Play (Variables|Default|GetOuverture-porte) 0.0)
    (Variables|Default|SetRasLeCulDesBoolean true)
    (Rendering|Material|SetMaterial (Variables|Default|GetSphere) 0 "/Game/Materials/M_LumièrePorte_Inst.M_LumièrePorte_Inst")
    (bind _newtrack_0 (Timeline|Open Play)
      (:Update
        (Transformation|SetRelativeLocation _sm_door_l_staticmeshcomponent0 (Math|Vector|MakeVector (.x _relativelocation) (.y _relativelocation) (* _newtrack_0 3.3e+02)) false false)))))

(event EventBeginPlay
  (Components|Timeline|SetPlayRate (Variables|Default|GetOpen) 0.5))

(fn ConstructionScript)

(fn CanOpen?
  (for _array_element (Variables|Default|GetButton)
    (if (not (Variables|/Game/Blueprints/Objet_Interactable/BP_Button.BP_Button_C|GetActivated _array_element))
      (return false)))
  (return true))

(fn Ref)