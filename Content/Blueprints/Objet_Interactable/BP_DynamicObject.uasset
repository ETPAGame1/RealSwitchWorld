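; Interactable mesh object that belongs to the Light world, the Dark world or both, and toggles presence as the player switches worlds.
; Construction applies the mesh, caches materials and makes LinkedObjects references mutual.
; SwitchingWorld swaps collision and original or invisible materials for single-world objects, unless frozen.
; CallFreeze spreads to linked objects, highlights via custom depth stencil, then resyncs to the player's world after FreezeSeconds.
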(event EventCallFreeze
  (bind _staticmesh (Variables|Default|GetStaticMesh))
  (bind _staticmesh_2 (Variables|Default|GetStaticMesh))
  (if (not (Variables|Default|GetFreeze))
    (Variables|Default|SetFreeze true)
    (for _array_element (Variables|Default|GetLinkedObjects)
      (Default|CallFreeze _array_element))
    (Rendering|SetRenderCustomDepth _staticmesh true)
    (Rendering|SetCustomDepthStencilValue _staticmesh 2)
    (Utilities|FlowControl|RetriggerableDelay (Variables|Default|GetFreezeSeconds))
    (Variables|Default|SetFreeze false)
    (CallFunction|SwitchingWorld (Variables|/Game/Blueprints/BP_FirstPersonCharacter.BP_FirstPersonCharacter_C|GetIsInLightLevel? (.AsBP%20First%20Person%20Character (Utilities|Casting|CastToBP_FirstPersonCharacter (Game|GetPlayerCharacter 0)))))
    (Rendering|SetRenderCustomDepth _staticmesh_2 false)
    (Rendering|SetCustomDepthStencilValue _staticmesh_2 0)))

(event EventSwitchingWorld
  (params (Light :type Boolean))
  (if (not (Variables|Default|GetFreeze))
    (switch Utilities|FlowControl|Switch|SwitchonEnum_Worlds (Variables|Default|GetWorld)
      (:NewEnumerator0
        _)
      (:NewEnumerator1
        _))
    (Collision|SetCollisionEnabled (Variables|Default|GetStaticMesh) (select (== (Utilities|Enum|Equal(Enum) (Variables|Default|GetWorld) "NewEnumerator0") Light) "QueryAndPhysics" "NoCollision"))
    (for _index (range 0 (Rendering|Material|GetNumMaterials (Variables|Default|GetStaticMesh)))
      (Rendering|Material|SetMaterial (Variables|Default|GetStaticMesh) _index (select (== (Utilities|Enum|Equal(Enum) (Variables|Default|GetWorld) "NewEnumerator0") Light) (Utilities|Array|Get(acopy) (Variables|Default|GetinitialMaterials) _index) (Variables|Default|GetMatInvisible))))))

(fn ConstructionScript
  (Utilities|FlowControl|Sequence
    (:then_0
      ;[1 1 1] SwitchMesh
      (Components|StaticMesh|SetStaticMesh (Variables|Default|GetStaticMesh) (Variables|Default|Getmesh)))
    (:then_1
      ;[1 1 1] StockMaterials
      (switch Utilities|FlowControl|Switch|SwitchonEnum_Worlds (Variables|Default|GetWorld)
        (:NewEnumerator0
          _)
        (:NewEnumerator1
          _))
      (Collision|SetCollisionEnabled (Variables|Default|GetStaticMesh) (Utilities|Select :Index (Variables|Default|GetWorld) :NewEnumerator0 "QueryAndPhysics" :NewEnumerator1 "NoCollision" :NewEnumerator2 "QueryAndPhysics"))
      (bind _returnvalue (Rendering|Material|CreateDynamicMaterialInstance (Utilities|Select :Index (Variables|Default|GetWorld) :NewEnumerator0 "/Game/Materials/M_OnVerraBien_Inst1.M_OnVerraBien_Inst1" :NewEnumerator1 "/Game/Materials/M_OnVerraBien_Inst.M_OnVerraBien_Inst" :NewEnumerator2 "/Engine/MapTemplates/Materials/BasicAsset01.BasicAsset01") "None" "None" :!class /Script/Engine.KismetMaterialLibrary))
      (Variables|Default|SetMatInvisible _returnvalue)
      (Variables|Default|SetinitialMaterials (Rendering|Material|GetMaterials (Variables|Default|GetStaticMesh)))
      (for _index (range 0 (Rendering|Material|GetNumMaterials (Variables|Default|GetStaticMesh)))
        (Rendering|Material|SetMaterial (Variables|Default|GetStaticMesh) _index (Utilities|Select :Index (Variables|Default|GetWorld) :NewEnumerator0 (Utilities|Array|Get(acopy) (Variables|Default|GetinitialMaterials) _index) :NewEnumerator1 (Variables|Default|GetMatInvisible) :NewEnumerator2 (Utilities|Array|Get(acopy) (Variables|Default|GetinitialMaterials) _index)))))
    (:then_2
      (if (not (== (Utilities|Array|LastIndex (Variables|Default|GetLinkedObjects)) 0))
        (for _array_element (Variables|Default|GetLinkedObjects)
          (if (not (Utilities|Array|ContainsItem (Variables|BP_DynamicObject_C|GetLinkedObjects _array_element) self))
            (Utilities|Array|Add (Variables|BP_DynamicObject_C|GetLinkedObjects _array_element) self)))))))