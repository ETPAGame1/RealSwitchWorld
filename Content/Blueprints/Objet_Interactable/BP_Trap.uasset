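; BP_Trap is an interactable object that slides its door mesh vertically once every linked button is activated.
; ButtonInteract calls CanOpen, which loops over the Button array and fails on any inactive entry.
; On success it sets a flag and plays the Open timeline, slowed to half rate at BeginPlay, to drive the mesh's relative Z while keeping X and Y.
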(event EventBeginPlay
  (Components|Timeline|SetPlayRate (Variables|Default|GetOpen) 0.5))

(event EventButtonInteract
  (bind _sm_door_l_staticmeshcomponent0 (Variables|Default|GetSM_Door_L_StaticMeshComponent0))
  (bind _relativelocation (Variables|/Script/Engine.SceneComponent|GetRelativeLocation _sm_door_l_staticmeshcomponent0))
  (bind _m_enbatslescouilles (CallFunction|CanOpen?))
  (if _m_enbatslescouilles
    (Variables|Default|SetOuais true)
    (bind _newtrack_0 (Timeline|Open Play)
      (:Update
        (Transformation|SetRelativeLocation _sm_door_l_staticmeshcomponent0 (Math|Vector|MakeVector (.x _relativelocation) (.y _relativelocation) (* _newtrack_0 2e+02)) false false)))))

(fn ConstructionScript)

(fn CanOpen?
  (for _array_element (Variables|Default|GetButton)
    (if (not (Variables|/Game/Blueprints/Objet_Interactable/BP_Button.BP_Button_C|GetActivated _array_element))
      (return false)))
  (return true))