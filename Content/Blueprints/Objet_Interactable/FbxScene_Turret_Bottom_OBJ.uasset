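; Laser turret that fires a beam each Tick, bouncing off mirrors, if all linked buttons are active at BeginPlay.
; SpawnLaser line-traces and recursively reflects off BP_Mirror hits, reusing one BP_Laser per segment and ending surplus ones.
; BPI_Interact hits receive laser on/off messages, tracked through a single CurrentInteracted that clears when none is hit.
; ButtonInteract is empty and the delayed shutdown logic is unconnected, so firing never stops.
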(event EventBeginPlay
  (bind _m_enbatslescouilles (CallFunction|CanOpen?))
  (if _m_enbatslescouilles
    (Variables|Default|SetFiring true)
    (Components|Activation|Activate (Variables|Default|GetNS_Sparks) false)))

(event EventTick
  (params (DeltaSeconds :type Float%20%28single-precision%29))
  (bind _spawnlaserlocation (Variables|Default|GetSpawnLaserLocation))
  (if (Variables|Default|GetFiring)
    (CallFunction|SpawnLaser (Transformation|GetSocketLocation (Variables|Default|GetTurret_Bottom_001) "EndLaser") (+ (Transformation|GetWorldLocation _spawnlaserlocation) (* (Math|Vector|GetForwardVector _spawnlaserlocation) (Variables|Default|GetRaycastDist))) self)
    (Variables|Default|GetCurrentInteracted
      (:then
        (Utilities|FlowControl|Sequence
          (:then_0
            (if (not (Variables|Default|GetAtleastOne))
              (Class|BPIInteract|LaserInteract(Message) (Variables|Default|GetCurrentInteracted) false)
              (Variables|Default|SetCurrentInteracted 0)))
          (:then_1
            (Variables|Default|SetAtleastOne false))))
      (:else))))

(event EventButtonInteract)

(fn ConstructionScript)

(fn SpawnLaser
  (params (staaart :type Vector) (eeend :type Vector) (Last%20Actor :type Actor%20Object%20Reference) (iindex :type Integer))
  (bind _lasers (Variables|Default|GetLasers))
  (bind _lasers_2 (Variables|Default|GetLasers))
  (bind _output (Utilities|Array|Get(acopy) _lasers_2 iindex))
  (bind (_outhit _returnvalue) (Collision|LineTraceByChannel staaart eeend "TraceTypeQuery3" false (Utilities|Array|MakeArray Last%20Actor) "ForOneFrame"))
  (Utilities|IsValid (Utilities|Array|Get(acopy) (Variables|Default|GetLasers) iindex)
    (:Is%20Valid
      _)
    (:Is%20Not%20Valid
      (bind _returnvalue_2 (Game|SpawnActorfromClass "/Game/Blueprints/BP_Laser.BP_Laser_C" (Math|Transform|MakeTransform "0, 0, 0" "0, 0, 0" "1.000000,1.000000,1.000000") "Undefined" 0 0))
      (Utilities|Array|SetArrayElem _lasers_2 iindex _returnvalue_2 true)))
  (Variables|/Game/Blueprints/BP_Laser.BP_Laser_C|SetStartLocation _output (.tracestart _outhit))
  (Variables|/Game/Blueprints/BP_Laser.BP_Laser_C|SetEndLocation _output (select _returnvalue (.impactpoint _outhit) (.traceend _outhit)))
  (if (.bblockinghit _outhit)
    (if (Utilities|DoesObjectImplementInterface (.hitactor _outhit) "/Game/Blueprints/BPI_Interact.BPI_Interact_C")
      (Variables|Default|SetAtleastOne true)
      (Variables|Default|GetCurrentInteracted
        (:then
          (if (!= (Variables|Default|GetCurrentInteracted) (.hitactor _outhit))
            (Class|BPIInteract|LaserInteract(Message) (Variables|Default|GetCurrentInteracted) false)
            (Variables|Default|SetCurrentInteracted (.hitactor _outhit))
            (Class|BPIInteract|LaserInteract(Message) (Variables|Default|GetCurrentInteracted) true :!label _label)
            (Utilities|Casting|CastToBP_Mirror (.hitactor _outhit) :!label _label_2
              (:then
                (CallFunction|SpawnLaser (.impactpoint _outhit) (+ (.impactpoint _outhit) (* (Math|Vector|MirrorVectorbyNormal (Math|Vector|GetUnitDirection(Vector) (.tracestart _outhit) (.traceend _outhit)) (.normal _outhit)) (Variables|Default|GetRaycastDist))) (.hitactor _outhit) (+ iindex 1)))
              (:CastFailed
                (bind _index (Utilities|FlowControl|ForLoopwithBreak (+ iindex 1) (Utilities|Array|LastIndex (Variables|Default|GetLasers)) :!label _label_3)
                  (:LoopBody
                    (Utilities|IsValid (Utilities|Array|Get(acopy) _lasers _index)
                      (:Is%20Valid
                        (Default|End (Utilities|Array|Get(acopy) _lasers _index))
                        (Utilities|Array|SetArrayElem _lasers _index 0)))))))))
        (:else
          (Variables|Default|SetCurrentInteracted (.hitactor _outhit))
          (goto _label)))
      (else
        (goto _label_2)))
    (else
      (goto _label_3))))

(fn CanOpen?
  (for _array_element (Variables|Default|GetButton)
    (if (not (Variables|/Game/Blueprints/Objet_Interactable/BP_Button.BP_Button_C|GetActivated _array_element))
      (return false)))
  (return true))