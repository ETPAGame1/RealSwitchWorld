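; BP_DynamicNeon is a neon light prop that changes its look when the world switches between light and non-light states.
; The SwitchingWorld event uses its Light flag to swap the emissive-slot material on five static meshes and turn the RectLight red-orange or blue.
; The Construction Script applies a warm red-orange color and the Light-state material as the default look.
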(event EventBeginPlay)

(event Collision|EventActorBeginOverlap
  (params (OtherActor :type Actor%20Object%20Reference)))

(event EventTick
  (params (DeltaSeconds :type Float%20%28single-precision%29)))

(event EventSwitchingWorld
  (params (Light :type Boolean))
  (Rendering|Material|SetMaterial (Variables|Default|GetStaticMesh4) 2 (select Light "/Game/StarterBundle/ModularScifiProps/Materials/MI_Light_White_2.MI_Light_White_2" "/Game/StarterBundle/ModularScifiProps/Materials/MI_Light_White.MI_Light_White"))
  (Rendering|Components|Light|SetLightColor (Variables|Default|GetRectLight) (select Light "(R=1.000000,G=0.274677,B=0.194618,A=1.000000)" "(R=0.000000,G=0.200000,B=1.000000,A=1.000000)") true))

(fn ConstructionScript
  (Rendering|Components|Light|SetLightColor (Variables|Default|GetRectLight) "(R=0.527115,G=0.035601,B=0.000000,A=1.000000)" true)
  (Rendering|Material|SetMaterial (Variables|Default|GetStaticMesh1) 2 "/Game/StarterBundle/ModularScifiProps/Materials/MI_Light_White_2.MI_Light_White_2"))