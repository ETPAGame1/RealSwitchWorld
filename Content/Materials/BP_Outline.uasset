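; BP_Outline is a Blueprint that adds and removes an outline mesh over its StaticMesh component on demand.
; Createoutline spawns an unattached mesh component at that component's world transform, assigns Mesh, and drives Color and Scale through a dynamic instance of its first material.
; DeleteOutline destroys the spawned component, and the HasOutline flag prevents duplicate outlines.
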(event Custom|Create%20outline
  (if (not (Variables|Default|GetHas%20outline))
    (bind _returnvalue (AddComponent|AddStaticMeshComponent true (Transformation|GetWorldTransform (Variables|Default|GetStaticMesh))))
    (bind _output_get (Variables|Default|SetMashComponent _returnvalue))
    (Components|StaticMesh|SetStaticMesh _output_get (Variables|Default|GetMesh))
    (bind _returnvalue_2 (Rendering|Material|CreateDynamicMaterialInstance _output_get 0 0 "None" :!class /Script/Engine.PrimitiveComponent))
    (Rendering|Material|SetVectorParameterValue _returnvalue_2 "Color" (Variables|Default|GetColor) :!class /Script/Engine.MaterialInstanceDynamic)
    (Rendering|Material|SetScalarParameterValue _returnvalue_2 "Scale" (Variables|Default|GetScale) :!class /Script/Engine.MaterialInstanceDynamic)
    (Variables|Default|SetHas%20outline true)))

(event Custom|Delete%20Outline
  (bind _mashcomponent (Variables|Default|GetMashComponent))
  (Utilities|IsValid _mashcomponent
    (:Is%20Valid
      (Components|DestroyComponent _mashcomponent)
      (Variables|Default|SetHas%20outline false))))

(fn ConstructionScript)